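; BP_Obstacle is a level-generation obstacle that knocks the player down on contact.
; The construction script randomly sizes its box collider to either tall or short obstacle dimensions.
; When the box is hit by BP_PlayerSkeleton, it calls FallDown on that player; a random static mesh swap is present but disconnected.
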(event `self.Box.OnComponentHit`
  (params (HitComponent :type "PrimitiveComponent Object Reference") (OtherActor :type "Actor Object Reference") (OtherComp :type "PrimitiveComponent Object Reference") (NormalImpulse :type "Vector Structure") (Hit :type "HitResult Structure (by ref)"))
  ;[1 1 1] If the player hits an obstacle, trigger an event in the player blueprint (BP_PlayerSkeleton)
  (bind _asbp_player_skeleton (cast `/Game/PlayerCharacter/Blueprints/BP_PlayerSkeleton` OtherActor))
  (`/Game/PlayerCharacter/Blueprints/BP_PlayerSkeleton.Fall Down` _asbp_player_skeleton))

(fn `UserConstructionScript`
  (`BoxComponent.SetBoxExtent` (`self.Box`) (select `bool` (`KismetMathLibrary.RandomBool`) :`false` (`self.shortObstacleDimensions`) :`true` (`self.tallObstacleDimensions`)) true))