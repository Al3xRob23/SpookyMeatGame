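; BP_Graveyard is a graveyard piece for level generation, built with six fence meshes.
; Its construction script varies the fences by adding a random negative offset to each one's world Z scale, leaving X and Y unchanged.
; GetAttachTransform and GetTileType suggest a tile interface for the generator, but both graphs are empty here.
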(fn `getAttachTransform`)

(fn `getTileType`)

(fn `UserConstructionScript`
  (for _array_element (`|MakeArray` (`self.FenceMesh1`) (`self.FenceMesh2`) (`self.FenceMesh3`) (`self.FenceMesh4`) (`self.FenceMesh5`) (`self.FenceMesh6`))
    (bind (_returnvalue_x _returnvalue_y _returnvalue_z) (`KismetMathLibrary.BreakVector` (`SceneComponent.K2_GetComponentScale` _array_element)))
    (`SceneComponent.SetWorldScale3D` _array_element (`KismetMathLibrary.MakeVector` _returnvalue_x _returnvalue_y (+ _returnvalue_z (`KismetMathLibrary.RandomFloatInRange` -6.0 -0.005))))))