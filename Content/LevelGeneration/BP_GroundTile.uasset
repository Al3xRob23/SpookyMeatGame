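; Ground tile for the skeleton runner's endless level, randomly populating itself and chaining to the next tile.
; BeginPlay spawns one random meat pickup, two same-height graves and one moving grave at random marker points.
; When the player overlaps EndOfTile, it notifies the player, has the game mode spawn another tile, then destroys itself after a delay.
; The construction script randomizes fence Z scale, and GetAttachTransform exposes the arrow's attach point.
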(event `self.ReceiveBeginPlay`
  (bind _returnvalue (`SceneComponent.K2_GetComponentToWorld` (`|GetArrayItem` (`|MakeArray` (`self.PickupLocation1`) (`self.PickupLocation2`) (`self.PickupLocation3`)) (`KismetMathLibrary.RandomIntegerInRange` 0 2))))
  (bind _returnvalue_2 (`SceneComponent.K2_GetComponentToWorld` (`|GetArrayItem` (`|MakeArray` (`self.MovingObstacleLocation1`) (`self.MovingObstacleLocation2`)) (`KismetMathLibrary.RandomIntegerInRange` 0 1))))
  (bind _returnvalue_3 (`SceneComponent.K2_GetComponentToWorld` (`|GetArrayItem` (`|MakeArray` (`self.ObstacleLocation1`) (`self.ObstacleLocation2`) (`self.ObstacleLocation3`) (`self.ObstacleLocation4`)) (`KismetMathLibrary.RandomIntegerInRange` 0 3))))
  ;[1 1 1] Spawn BP_MeatPickup at varied locations
  (`|ExecutionSequence`
    (:`then_0`
      (if (`KismetMathLibrary.RandomBool`)
        (if (`KismetMathLibrary.RandomBool`)
          (`|SpawnActorFromClass` "/Game/LevelGeneration/Pickups/BP_MeatPickup2.BP_MeatPickup2_C" _returnvalue "Undefined" "OverrideRootScale" null null)
          (else
            (`|SpawnActorFromClass` "/Game/LevelGeneration/Pickups/BP_MeatPickup4.BP_MeatPickup4_C" _returnvalue "Undefined" "OverrideRootScale" null null)))
        (elif (`KismetMathLibrary.RandomBool`)
          (`|SpawnActorFromClass` "/Game/LevelGeneration/Pickups/BP_MeatPickup3.BP_MeatPickup3_C" _returnvalue "Undefined" "OverrideRootScale" null null)
          (else
            (`|SpawnActorFromClass` "/Game/LevelGeneration/Pickups/BP_MeatPickup.BP_MeatPickup_C" _returnvalue "Undefined" "OverrideRootScale" null null)))))
    (:`then_1`
      ;[1 1 1] Spawn an obstacle at the chosen location
      (if (`KismetMathLibrary.RandomBool`)
        (`|SpawnActorFromClass` "/Game/LevelGeneration/BP_GraveShort.BP_GraveShort_C" _returnvalue_3 "Undefined" "OverrideRootScale" null null)
        (`|SpawnActorFromClass` "/Game/LevelGeneration/BP_GraveShort.BP_GraveShort_C" _returnvalue_3 "Undefined" "OverrideRootScale" null null)
        (else
          (`|SpawnActorFromClass` "/Game/LevelGeneration/BP_GraveTall.BP_GraveTall_C" _returnvalue_3 "Undefined" "OverrideRootScale" null null)
          (`|SpawnActorFromClass` "/Game/LevelGeneration/BP_GraveTall.BP_GraveTall_C" _returnvalue_3 "Undefined" "OverrideRootScale" null null))))
    (:`then_2`
      ;[1 1 1] Spawn an obstacle at the chosen location
      (if (`KismetMathLibrary.RandomBool`)
        (`|SpawnActorFromClass` "/Game/LevelGeneration/BP_MovingGraveShort.BP_MovingGraveShort_C" _returnvalue_2 "Undefined" "OverrideRootScale" null null)
        (else
          (`|SpawnActorFromClass` "/Game/LevelGeneration/BP_MovingGraveTall.BP_MovingGraveTall_C" _returnvalue_2 "Undefined" "OverrideRootScale" null null))))))

(event `self.EndOfTile.OnComponentBeginOverlap`
  (params (OverlappedComponent :type "PrimitiveComponent Object Reference") (OtherActor :type "Actor Object Reference") (OtherComp :type "PrimitiveComponent Object Reference") (OtherBodyIndex :type Integer) (bFromSweep :type Boolean) (SweepResult :type "HitResult Structure (by ref)"))
  ;[1 1 1] If the player collided with the End-of-tile collider, trigger an event in the player blueprint (BP_PlayerSkeleton)
  (bind _asbp_player_skeleton (cast `/Game/PlayerCharacter/Blueprints/BP_PlayerSkeleton` OtherActor))
  (`/Game/PlayerCharacter/Blueprints/BP_PlayerSkeleton.CompletedOneTile` _asbp_player_skeleton)
  ;[1 1 1] Once the player has passed over a tile, spawn a new one ahead of them...
  (bind _asgm_skeleton_runner_game_mode (cast `/Game/MapAndGameMode/GM_SkeletonRunnerGameMode` (`GameplayStatics.GetGameMode`)))
  (`/Game/MapAndGameMode/GM_SkeletonRunnerGameMode.Spawn Ground Tile` _asgm_skeleton_runner_game_mode)
  ;[1 1 1] ...then destroy the old one
  (`KismetSystemLibrary.Delay` 2.0) ; This delay prevents the tile disappearing while on-screen
  (`self.K2_DestroyActor`))

(fn `getAttachTransform`
  (returns (ReturnValue :type "Transform Structure"))
  (return (`SceneComponent.K2_GetComponentToWorld` (`self.AttachPointArrow`))))

(fn `getTileType`)

(fn `UserConstructionScript`
  (for _array_element (`|MakeArray` (`self.FenceMesh1`) (`self.FenceMesh2`) (`self.FenceMesh3`) (`self.FenceMesh4`) (`self.FenceMesh5`) (`self.FenceMesh6`))
    (bind (_returnvalue_x _returnvalue_y _returnvalue_z) (`KismetMathLibrary.BreakVector` (`SceneComponent.K2_GetComponentScale` _array_element)))
    (`SceneComponent.SetWorldScale3D` _array_element (`KismetMathLibrary.MakeVector` _returnvalue_x _returnvalue_y (+ _returnvalue_z (`KismetMathLibrary.RandomFloatInRange` -6.0 -0.005))))))