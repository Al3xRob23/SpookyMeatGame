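; Player character for a skeleton endless runner that auto-runs forward after Space starts the run, with lateral steering and jumping.
; A skeleton state drives movement on Tick and is pushed to the animation Blueprint.
; Each completed tile raises walk speed and score, while high score and meat pickups persist in the game instance.
; Falling down ends the run and reloads PersistentMap after a short delay to reset everything.
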(event `self.ReceiveBeginPlay`
  ;[1 1 1] Spawning and starting the run
  ;;[1 1 1] Initialise variables and set player to "Idle
  (bind _asabp_player_skeleton (cast `/Game/PlayerCharacter/Blueprints/ABP_PlayerSkeleton` (`SkeletalMeshComponent.GetAnimInstance` (`self.Mesh`))))
  (set `self.AnimationBlueprintReference` _asabp_player_skeleton)
  (bind _asgm_skeleton_runner_game_mode (cast `/Game/MapAndGameMode/GM_SkeletonRunnerGameMode` (`GameplayStatics.GetGameMode`)))
  (set `self.gameModeReference` _asgm_skeleton_runner_game_mode)
  (bind _asbp_skeleton_runner_game_instance (cast `/Game/MapAndGameMode/BP_SkeletonRunnerGameInstance` (`GameplayStatics.GetGameInstance`)))
  (bind _output_get (set `self.gameInstanceRef` _asbp_skeleton_runner_game_instance))
  (`self.setHighScore` (`/Game/MapAndGameMode/BP_SkeletonRunnerGameInstance.HighScore` _output_get))
  (`self.setPickupAmount` (`/Game/MapAndGameMode/BP_SkeletonRunnerGameInstance.MeatCollected` _output_get))
  (set `self.playerControllerRef` (`GameplayStatics.GetPlayerController` 0)))

(event `Key|SpaceBar`
  (params (Key :type "Key Structure"))
  ;[1 1 1] Spawning and starting the run
  ;;[1 1 1] Start the player running once they have spawned
  (:`Pressed`
    (if (not (`self.runStarted`))
      (set `self.runStarted` true)
      (`ActorComponent.K2_DestroyComponent` (`self.startRunText`))
      (`self.Changed State` "NewEnumerator1")
      (`self.SetActorTickEnabled` true))))

(event `self.ReceiveTick`
  (params (DeltaSeconds :type "Float (single-precision)"))
  ;[1 1 1] Movement Controls
  (switch `/Game/PlayerCharacter/Blueprints/E_PlayerSkeletonStates` (`self.currentSkeletonState`)
    (:`NewEnumerator1`
      ;;[1 1 1] Move the player forward constantly (if they are running or jumping)
      (`self.AddMovementInput` (`KismetMathLibrary.GetForwardVector` (`KismetMathLibrary.MakeRotator` 0.0 0.0 (.yaw (`self.GetControlRotation`)))) (`self.RunSpeed`) :!label _label))
    (:`NewEnumerator2`
      (if (`NavMovementComponent.IsMovingOnGround` (`self.CharacterMovement`))
        (set `self.inAir` false)
        (`self.Changed State` "NewEnumerator1")
        (goto _label)))
    (:`NewEnumerator3`
      (goto _label))))

(event `InputAxis|MoveRight` :overrideparent false
  (params (AxisValue :type "Float (single-precision)"))
  ;[1 1 1] Movement Controls
  ;;[1 1 1] Turn the player when they press left and right (set to A and D in project settings)
  (if (`self.runStarted`)
    (if (not (`self.inAir`))
      (`self.AddMovementInput` (`KismetMathLibrary.GetRightVector` (`KismetMathLibrary.MakeRotator` 0.0 0.0 (.yaw (`self.GetControlRotation`)))) AxisValue))))

(event `InputAction|Jump` :overrideparent false
  (params (Key :type "Key Structure"))
  ;[1 1 1] Movement Controls
  ;;[1 1 1] Jump when the player presses "jump" (set to spacebar in project settings) , unless the run hasn't started yet.
  (:`Pressed`
    (if (`self.runStarted`)
      (set `self.inAir` true)
      (`self.Jump`)
      (`self.Changed State` "NewEnumerator2")))
  (:`Released`
    (`self.StopJumping`)))

(event `Changed State`
  (params (NewState :type "/Game/PlayerCharacter/Blueprints/E_PlayerSkeletonStates Enum" :default "NewEnumerator0"))
  ;[1 1 1] When the skeleton changes state (eg. running to jumping) we also update this in the Animation blueprint, so the animation changes appropriately
  (bind _output_get (set `self.currentSkeletonState` NewState))
  (set `/Game/PlayerCharacter/Blueprints/ABP_PlayerSkeleton.skeletonState` _output_get (`self.AnimationBlueprintReference`)))

(event `CompletedOneTile`
  (bind _charactermovement (`self.CharacterMovement`))
  ;[1 1 1] After the player has run across a tile, we increase the speed and give them a point.
  (set `CharacterMovementComponent.MaxWalkSpeed` (+ (`CharacterMovementComponent.MaxWalkSpeed` _charactermovement) 30.0) _charactermovement)
  (`self.increaseCurrentScore`))

(event `Fall Down`
  ;[1 1 1] This is the "fail state". Triggered when the player hits an obstacle
  (`self.Changed State` "NewEnumerator3")
  (set `self.runStarted` false)
  (`KismetSystemLibrary.Delay` 1.5)
  ;[1 1 1] Loading the map is an easy way to reset everything
  (`GameplayStatics.OpenLevel` "PersistentMap" true (`KismetSystemLibrary.GetDisplayName` (`self.gameModeReference`))))

(fn `checkPickupAmount`
  (if (>= (`self.meatCollected`) (`/Game/PlayerCharacter/Blueprints/BP_MeatStoreUI.amountNeeded` (`self.ArmL_Button`)))
    (set `self.meatCollected` (- (`/Game/PlayerCharacter/Blueprints/BP_MeatStoreUI.amountNeeded` (`self.ArmL_Button`)) (`self.meatCollected`)))))

(fn `decreasePickupAmount`
  (params (`amount to decrease by` :type Integer))
  (bind _gameinstanceref (`self.gameInstanceRef`))
  (bind _output_get (set `/Game/MapAndGameMode/BP_SkeletonRunnerGameInstance.MeatCollected` (- (`/Game/MapAndGameMode/BP_SkeletonRunnerGameInstance.MeatCollected` _gameinstanceref) `amount to decrease by`) _gameinstanceref)))

(fn `increaseCurrentScore`
  (`|ExecutionSequence`
    (:`then_0`
      (bind _result (`/Engine/EditorBlueprintResources/StandardMacros.IncrementInt` (`self.CurrentScore`))))
    (:`then_1`
      (if (> (`self.CurrentScore`) (`self.HighScore`))
        (`self.setHighScore` (`self.CurrentScore`))))))

(fn `increasePickupAmount`
  (params (MeatCollected :type Integer))
  (bind _result (`/Engine/EditorBlueprintResources/StandardMacros.IncrementInt` (`/Game/MapAndGameMode/BP_SkeletonRunnerGameInstance.MeatCollected` (`self.gameInstanceRef`)))))

(fn `resetCurrentScore`
  (set `self.CurrentScore` 0))

(fn `setHighScore`
  (params (HighScore :type Integer))
  (bind _output_get (set `self.HighScore` HighScore))
  (bind _output_get_2 (set `/Game/MapAndGameMode/BP_SkeletonRunnerGameInstance.HighScore` _output_get (`self.gameInstanceRef`))))

(fn `setPickupAmount`
  (params (pickupAmount :type Integer)))

(fn `UserConstructionScript`)