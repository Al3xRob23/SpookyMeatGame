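; BP_Thunder is a lightning effect actor that repeatedly flashes a strike at random intervals of a few seconds.
; Each strike plays the ThunderStrike timeline, driving the Y and emissive material parameters on ThunderPlane.
; Shortly afterwards it briefly spikes manual exposure compensation on the PostProcessVolume found at BeginPlay, then restores the saved value.
; Both exposure writes assign a newly built settings struct to the volume.
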(event `self.ReceiveBeginPlay`
  (bind _pp_volume (`self.PP_Volume`))
  (bind _returnvalue (`GameplayStatics.GetActorOfClass` "/Script/Engine.PostProcessVolume"))
  (set `self.PP_Volume` _returnvalue)
  (`KismetSystemLibrary.Delay` (`KismetMathLibrary.RandomFloatInRange` 1.0 4.0) :!label _label)
  (`self.Strike`)
  (`KismetSystemLibrary.Delay` 0.2)
  (bind _output_get (set `self.Original Exposure Compensation` (`.AutoExposureBias` (break `PostProcessSettings` (`PostProcessVolume.Settings` _pp_volume)))))
  (set `PostProcessVolume.Settings` (make `PostProcessSettings` :`AutoExposureMethod` "AEM_Manual" :`AutoExposureBias` 10.0) _pp_volume)
  (`KismetSystemLibrary.Delay` 0.1)
  (set `PostProcessVolume.Settings` (make `PostProcessSettings` :`AutoExposureMethod` "AEM_Manual" :`AutoExposureBias` _output_get) _pp_volume)
  (goto _label))

(event `Strike`
  (bind (_direction _y) (`Timeline|ThunderStrike` :!via `PlayFromStart`)
    (:`Update`
      (`MeshComponent.SetScalarParameterValueOnMaterials` (`self.ThunderPlane`) "Y" _y)
      (`MeshComponent.SetScalarParameterValueOnMaterials` (`self.ThunderPlane`) "Emmisive" (* (+ _y 1.0) 50.0)))))

(fn `UserConstructionScript`)